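; Standard_Object is a placeable shape actor labeled with a random letter or digit, configured through its Activate event.
; Activate moves it to a given location, applies a random yaw and scales the Shape component, leaving the Emergent input unused.
; It gives the shape a dynamic material with a random-hue color and tints the text with the inverse color for contrast.
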(event `Activate`
  (params (Location :type "Vector Structure") (Scale :type "Vector Structure") (Emergent :type Boolean))
  (bind (_r _g _b) (`KismetMathLibrary.BreakColor` (`self.Color`)))
  (`self.K2_SetActorLocation` Location)
  (`self.K2_SetActorRotation` (`KismetMathLibrary.MakeRotator` 0.0 0.0 (`KismetMathLibrary.RandomFloatInRange` 0.0 360.0)))
  (`SceneComponent.SetWorldScale3D` (`self.Shape`) Scale)
  (bind _returnvalue (`PrimitiveComponent.CreateDynamicMaterialInstance` (`self.Shape`) 0 "/Game/Materials/Standard_Object_Color.Standard_Object_Color" "None"))
  (set `self.Shape Dynamic Material Instance` _returnvalue)
  (`TextRenderComponent.K2_SetText` (`self.Letter`) (`KismetTextLibrary.Conv_StringToText` (select `int` (`KismetMathLibrary.RandomInteger` 36) :`0` "A" :`1` "B" :`2` "C" :`3` "D" :`4` "E" :`5` "F" :`6` "G" :`7` "H" :`8` "I" :`9` "J" :`10` "K" :`11` "L" :`12` "M" :`13` "N" :`14` "O" :`15` "P" :`16` "Q" :`17` "R" :`18` "S" :`19` "T" :`20` "U" :`21` "V" :`22` "W" :`23` "X" :`24` "Y" :`25` "Z" :`26` "0" :`27` "1" :`28` "2" :`29` "3" :`30` "4" :`31` "5" :`32` "6" :`33` "7" :`34` "8" :`35` "9")))
  (set `self.Color` (`KismetMathLibrary.MakeColor` 1.0))
  (`KismetMathLibrary.LinearColor_SetRandomHue` (`self.Color`))
  (`MaterialInstanceDynamic.SetVectorParameterValue` (`self.Shape Dynamic Material Instance`) "Color" (`self.Color`))
  (`TextRenderComponent.SetTextRenderColor` (`self.Letter`) (`KismetMathLibrary.Conv_LinearColorToColor` (`KismetMathLibrary.MakeColor` (- 1.0 _r) (- 1.0 _g) (- 1.0 _b)))))

(fn `UserConstructionScript`)