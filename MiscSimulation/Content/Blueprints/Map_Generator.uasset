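; Map generator Blueprint that builds a set of cylinders from the CylinderData array.
; BuildCylinders adds one Instanced Static Mesh component and an instance per entry, placed at its spawn point and scaled from radius and height.
; BuildInEditor selects whether this runs in the Construction Script or at BeginPlay.
; Only the BeginPlay path stores the resulting component in InstancedCylinders, when the build succeeds.
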(event `self.ReceiveBeginPlay`
  (if (not (`self.Build in Editor`))
    (bind (_success _instanced_cylinders) (`self.Build Cylinders`))
    (if _success
      (set `self.Instanced Cylinders` _instanced_cylinders))))

(fn `Build Cylinders`
  (returns (Success :type Boolean) (`Instanced Cylinders` :type "InstancedStaticMeshComponent Object Reference"))
  (locals (Cylinders :type "InstancedStaticMeshComponent Object Reference") (Pass :type Boolean :default false))
  (bind _output_get (set `local.Pass` (!= (`KismetArrayLibrary.Array_Length` (`self.Cylinder Data`)) 0)))
  (if _output_get
    (bind _returnvalue (`AddComponent|NODE_AddInstancedStaticMeshComponent-0`))
    (set `local.Cylinders` _returnvalue)
    (for _array_element (`self.Cylinder Data`)
      (bind (_cylinderspawnpoint _cylinderradius _cylinderheight) (break `/Game/zETC/Cyllinder_Struct` _array_element))
      (bind _returnvalue_2 (/ _cylinderradius 50.0))
      (`InstancedStaticMeshComponent.AddInstance` (`local.Cylinders`) (`KismetMathLibrary.MakeTransform` _cylinderspawnpoint (struct) (`KismetMathLibrary.MakeVector` _returnvalue_2 _returnvalue_2 (/ _cylinderheight 100.0))))))
  (return (`local.Pass`) (`local.Cylinders`)))

(fn `UserConstructionScript`
  (if (`self.Build in Editor`)
    (`self.Build Cylinders`)))